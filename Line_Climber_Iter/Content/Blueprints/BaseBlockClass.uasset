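; Base falling block for what appears to be a side-scroller, which kills the player when it lands on them.
; While interactable, Tick lowers the Cube by unswept world offsets at normal or bash speed; otherwise it disables physics simulation.
; On hit, a tagged player below the Cube and within its half-width on Y gets Die called.
; The Cube's own hit event only prints and sets a Hit flag.
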(event `self.ReceiveHit`
  (params (MyComp :type "PrimitiveComponent Object Reference") (Other :type "Actor Object Reference") (OtherComp :type "PrimitiveComponent Object Reference") (bSelfMoved :type Boolean) (HitLocation :type "Vector Structure") (HitNormal :type "Vector Structure") (NormalImpulse :type "Vector Structure") (Hit :type "HitResult Structure (by ref)"))
  ;[1 1 1] Kill player on collision from above
  (if (`self.ActorHasTag` Other (`self.PlayerTag`))
    (if (and (< (.z (`SceneComponent.K2_GetComponentLocation` OtherComp)) (.z (`SceneComponent.K2_GetComponentLocation` (`self.Cube`)))) (< (`KismetMathLibrary.Abs` (- (.y (`SceneComponent.K2_GetComponentLocation` OtherComp)) (.y (`SceneComponent.K2_GetComponentLocation` (`self.Cube`))))) (/ (.y (`.Max` (break `Box` (`StaticMesh.GetBoundingBox` (`StaticMeshComponent.StaticMesh` (`self.Cube`)))))) 2.0)))
      (bind _asside_scroller_character_no_cam (cast `/Game/Casey/SideScrollerCharacter_NoCam` Other)
        (:`then`
          (`/Game/Casey/SideScrollerCharacter_NoCam.Die` _asside_scroller_character_no_cam))
        (:`CastFailed`
          (`KismetSystemLibrary.PrintString` "A non-player character is tagged as a player"))))))

(event `self.ReceiveTick`
  (params (DeltaSeconds :type "Float (single-precision)"))
  (if (`self.IsInteractable`)
    (if (`self.IsBashing`)
      ;[1 1 1] Bash Drop
      (bind _output_get (set `self.DropSpeed` (`self.DropSpeedBash`)))
      (`SceneComponent.K2_AddWorldOffset` (`self.Cube`) (`KismetMathLibrary.MakeVector` 0.0 0.0 (* _output_get -1.0)) false false)
      (else
        ;[1 1 1] Normal Drop
        (bind _output_get_2 (set `self.DropSpeed` (`self.DropSpeedNormal`)))
        (`SceneComponent.K2_AddWorldOffset` (`self.Cube`) (`KismetMathLibrary.MakeVector` 0.0 0.0 (* _output_get_2 -1.0)) false false)))
    (else
      (`PrimitiveComponent.SetSimulatePhysics` (`self.Cube`) false))))

(event `self.Cube.OnComponentHit`
  (params (HitComponent :type "PrimitiveComponent Object Reference") (OtherActor :type "Actor Object Reference") (OtherComp :type "PrimitiveComponent Object Reference") (NormalImpulse :type "Vector Structure") (Hit :type "HitResult Structure (by ref)"))
  (`KismetSystemLibrary.PrintString` "Hit")
  (set `self.Hit` true))

(fn `UserConstructionScript`)